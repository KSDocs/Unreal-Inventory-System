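; Base weapon actor that a character picks up on overlap and fires with left mouse while aiming, automatic or single-shot.
; A Tick-fed gate and a delayed DoOnce pace shots, passing the local camera view through SetCameraServer before FireServer.
; Fire traces from the camera, then from the muzzle socket to that point to catch obstructions.
; It then plays effects, pushes simulating bodies and applies damage.
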(event OnComponentBeginOverlap(Sphere)
  (params (OverlappedComponent :type Primitive%20Component%20Object%20Reference) (OtherActor :type Actor%20Object%20Reference) (OtherComp :type Primitive%20Component%20Object%20Reference) (OtherBodyIndex :type Integer) (bFromSweep :type Boolean) (SweepResult :type Hit%20Result%20Structure%20%28by%20ref%29))
  (EventDispatchers|UnbindallEventsfromOnComponentBeginOverlap (Variables|Default|GetSphere))
  (Components|DestroyComponent (Variables|Default|GetSphere))
  (bind _ascharacter (Utilities|Casting|CastToCharacter OtherActor))
  (bind _output_get (Variables|Default|SetCharacter _ascharacter))
  (Actor|SetOwner (Components|GetOwner _output_get))
  (if (Pawn|IsLocallyControlled _output_get)
    (Input|EnableInput (Game|GetPlayerController 0))))

(event Custom|Fire
  (Development|PrintString "Fire")
  (Audio|PlaySoundatLocation (Variables|Default|GetWeaponSound) (Transformation|GetActorLocation) "0, 0, 0" 1.0 1.0 0.0 0 0 0 0)
  (Effects|SpawnEmitterAttached (Variables|Default|GetFlash%20Emitter) (Variables|Default|GetSkeletalMesh) "TIP")
  (bind (_location _hitactor _hitcomponent _bonename _impluse) (CallFunction|TraceCamera (Variables|Default|GetWeapon%20Range)))
  (bind (_location1 _hit_component1 _hit_actor1 _impulse1 _bone_name1) (CallFunction|TraceSocket _location _hitactor _hitcomponent _bonename _impluse))
  (Effects|SpawnEmitteratLocation (Variables|Default|GetEmitter%20Template) _location1)
  (CallFunction|ApplyPhysics _location1 _impulse1 _hit_component1 _bone_name1)
  (Game|Damage|ApplyDamage _hit_actor1 (Variables|Default|GetWeapon%20Damage) 0 (Variables|Default|GetCharacter)))

(event Custom|Set%20Camera%20Server
  (params (Camera%20Location :type Vector) (Camera%20Forward :type Vector))
  ;[0.15 0.15 0.15 0.5] Replicate Camera
  (CallFunction|SetCamera Camera%20Location Camera%20Forward))

(event Custom|SetCamera
  (params (Camera%20Location :type Vector) (Camera%20Forward :type Vector))
  ;[0.15 0.15 0.15 0.5] Replicate Camera
  (Variables|Default|SetCamera%20Location Camera%20Location)
  (Variables|Default|SetCamera%20Forward Camera%20Forward))

(event Custom|Fire%20Server
  (CallFunction|Fire))

(event EventTick
  (params (DeltaSeconds :type Float%20%28single-precision%29))
  (bind _returnvalue (Game|GetPlayerCameraManager 0))
  (Utilities|FlowControl|Gate true
    (:Exit
      (Utilities|FlowControl|DoOnce false :!label _label
        (:Completed
          (CallFunction|SetCameraServer (Transformation|GetActorLocation _returnvalue) (Transformation|GetActorForwardVector _returnvalue))
          (CallFunction|FireServer)
          (Utilities|FlowControl|Delay (Variables|Default|GetFireRate))
          (goto _label Reset))))))

(event Input|MouseEvents|LeftMouseButton
  (params (Key :type Key%20Structure :default "None"))
  (bind _returnvalue (Game|GetPlayerCameraManager 0))
  (:Pressed
    (bind _asbp_third_person_character (Utilities|Casting|CastToBP_ThirdPersonCharacter (Game|GetPlayerCharacter 0)))
    (if (Variables|/Game/ThirdPerson/Blueprints/BP_ThirdPersonCharacter.BP_ThirdPersonCharacter_C|GetAiming _asbp_third_person_character)
      (if (Variables|Default|GetAutomatic)
        (Utilities|FlowControl|Gate true) ; enters at Open
        (else
          (Utilities|FlowControl|DoOnce false :!label _label
            (:Completed
              (CallFunction|SetCameraServer (Transformation|GetActorLocation _returnvalue) (Transformation|GetActorForwardVector _returnvalue))
              (CallFunction|FireServer)
              (Utilities|FlowControl|Delay (Variables|Default|GetFireRate))
              (goto _label Reset)))))))
  (:Released
    (Utilities|FlowControl|Gate true) ; enters at Close
  ))

(fn ConstructionScript
  (Components|SkeletalMesh|SetSkeletalMeshAsset (Variables|Default|GetSkeletalMesh) (Variables|Default|GetMesh)))

(fn TraceCamera
  (params (WeaponRange :type Float%20%28double-precision%29))
  (bind _camera_location (Variables|Default|GetCamera%20Location))
  (bind _camera_forward (Variables|Default|GetCamera%20Forward))
  (bind _returnvalue (* _camera_forward WeaponRange))
  (bind _outhit (Collision|LineTraceByChannel _camera_location (+ _returnvalue _camera_location) "TraceTypeQuery3" false (Utilities|Array|MakeArray (Variables|Default|GetCharacter)) "None" true "(R=1.000000,G=0.000000,B=0.000000,A=1.000000)" "(R=0.000000,G=1.000000,B=0.000000,A=1.000000)" 1.0))
  (return (select (Utilities|Operators|EqualEqual :A (.Location (Collision|BreakHitResult _outhit))) (.TraceEnd (Collision|BreakHitResult _outhit)) (.Location (Collision|BreakHitResult _outhit))) (.HitActor (Collision|BreakHitResult _outhit)) (.HitComponent (Collision|BreakHitResult _outhit)) (.BoneName (Collision|BreakHitResult _outhit)) _returnvalue))

(fn TraceSocket
  (params (Location :type Vector) (Hit%20Actor :type Actor%20Object%20Reference) (Hit%20Component :type Primitive%20Component%20Object%20Reference) (Bone%20Name :type Name) (Impulse :type Vector))
  (bind _outhit (Collision|LineTraceByChannel (Transformation|GetSocketLocation (Variables|Default|GetSkeletalMesh) "TIP") Location "TraceTypeQuery3" false (Utilities|Array|MakeArray (Variables|Default|GetCharacter)) "None" true "(R=0.054045,G=0.000000,B=1.000000,A=1.000000)" "(R=0.000000,G=1.000000,B=0.000000,A=1.000000)" 1.0))
  (if (and (Class|KismetMathLibrary|NotEqualExactlyVectorVector "0, 0, 0" (.ImpactPoint (Collision|BreakHitResult _outhit))) (!= Hit%20Component (.HitComponent (Collision|BreakHitResult _outhit))))
    (return (.ImpactPoint (Collision|BreakHitResult _outhit)) (.HitComponent (Collision|BreakHitResult _outhit)) (.HitActor (Collision|BreakHitResult _outhit)) Impulse (.BoneName (Collision|BreakHitResult _outhit)))
    (else
      (return Location Hit%20Component Hit%20Actor Impulse Bone%20Name))))

(fn ApplyPhysics
  (params (Location :type Vector) (Impluse :type Vector) (Hit%20Component :type Primitive%20Component%20Object%20Reference) (Bone%20Name :type Name))
  (Utilities|IsValid Hit%20Component
    (:Is%20Valid
      (if (Physics|IsSimulatingPhysics Hit%20Component Bone%20Name)
        (Physics|AddImpulseatLocation Hit%20Component (* Impluse 2.0) Location Bone%20Name)))))